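; BP_Police is a police actor with a CanSeePlayer check for detecting the player pawn.
; The check combines distance, view angle from the forward vector, and a slightly raised Visibility line trace that must hit the player.
; Both distance and angle limits are zero, so as written it practically never returns true.
; The trace result is printed for debugging, and nothing in this file calls the check.
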(fn ConstructionScript)

(fn CanSeePlayer
  (bind _returnvalue (Game|Player|GetPlayerPawn 0))
  (bind _returnvalue_2 (Game|Player|GetPlayerPawn 0))
  (bind _outhit (Collision|LineTraceByChannel (+ (Transformation|GetActorLocation) "0.000000,0.000000,20.000000") (+ (Transformation|GetActorLocation _returnvalue_2) "0.000000,0.000000,20.000000") "TraceTypeQuery1" false (Utilities|Array|MakeArray self) "None"))
  (Development|PrintString (Utilities|String|ToString(Boolean) (== (.HitActor (Collision|BreakHitResult _outhit)) _returnvalue_2)))
  (return (Math|Boolean|ANDBoolean (<= (Transformation|GetDistanceTo _returnvalue) 0.0) (<= (Class|KismetMathLibrary|DegAcos (Math|Vector|DotProduct (Transformation|GetActorForwardVector) (Math|Vector|Normalize (- (Transformation|GetActorLocation _returnvalue) (Transformation|GetActorLocation))))) 0.0) (== (.HitActor (Collision|BreakHitResult _outhit)) _returnvalue_2))))