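; Player car pawn that drives via Enhanced Input, collects a level's goal number of coins and loses HP in crashes, reloading the level at zero.
; Tick applies movement input, eases rotation toward it and applies manual gravity through a swept offset.
; Fast side impacts with Police, Blocker or Border actors deal cooldown-gated damage.
; HP and coins feed the HUD; completion saves score through SaveSubsystem, then opens the next level or main menu.
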(event OnComponentHit(BoxCollision)
  (params (HitComponent :type Primitive%20Component%20Object%20Reference) (OtherActor :type Actor%20Object%20Reference) (OtherComp :type Primitive%20Component%20Object%20Reference) (NormalImpulse :type Vector :default "0, 0, 0") (Hit :type Hit%20Result%20Structure%20%28by%20ref%29))
  (bind _stats (Variables|Default|GetStats))
  (if (and (or (or (Actor|ActorHasTag OtherActor "Police") (Actor|ActorHasTag OtherActor "Blocker")) (Actor|ActorHasTag OtherActor "Border")) (Math|Boolean|ANDBoolean (< (.Z (Math|Vector|BreakVector (.ImpactNormal (Collision|BreakHitResult Hit)))) (Variables|/Game/Data/PDA_PlayerStats.PDA_PlayerStats_C|GetCollisionMaxNormalZ _stats)) (Variables|Default|GetCanTakeHit) (> (Math|Vector|VectorLength (Transformation|GetVelocity)) (Variables|/Game/Data/PDA_PlayerStats.PDA_PlayerStats_C|GetCollisionMinSpeed _stats))))
    (Variables|Default|SetCanTakeHit false)
    (Game|Damage|ApplyDamage self (Variables|/Game/Data/PDA_PlayerStats.PDA_PlayerStats_C|GetCollisionDamage _stats) 0 0)
    (Utilities|FlowControl|Delay (Variables|/Game/Data/PDA_PlayerStats.PDA_PlayerStats_C|GetHitCooldown _stats))
    (Variables|Default|SetCanTakeHit true)))

(event Custom|CollectCoin
  (bind _returnvalue (Subsystems|GetSaveSubsystem))
  (bind _output_get (Variables|Default|SetCoinsLeft (- (Variables|Default|GetCoinsLeft) 1)))
  (Variables|Default|SetScore (+ (Variables|Default|GetScore) (Variables|/Game/Data/PDA_ItemValues.PDA_ItemValues_C|GetCoinScore (Variables|Default|GetItems))))
  (Default|UpdateCoins (stale EventBeginPlay _output_get_2) _output_get)
  (if (<= (Variables|Default|GetCoinsLeft) 0)
    (Class|SaveSubsystem|CompleteLevel (Subsystems|GetSaveSubsystem) (Variables|/Script/Racescape.LevelData|GetLevelIndex (Variables|/Script/Racescape.SaveSubsystem|GetSelectedLevel _returnvalue)) (Variables|Default|GetScore))
    (Utilities|FlowControl|Delay (Variables|/Game/Data/PDA_PlayerStats.PDA_PlayerStats_C|GetLevelEndDelay (Variables|Default|GetStats)))
    (if (Utilities|IsValid (Variables|/Script/Racescape.LevelData|GetNextLevel (Variables|/Script/Racescape.SaveSubsystem|GetSelectedLevel _returnvalue)))
      (Variables|/Script/Racescape.SaveSubsystem|SetSelectedLevel _returnvalue (Variables|/Script/Racescape.LevelData|GetNextLevel (Variables|/Script/Racescape.SaveSubsystem|GetSelectedLevel _returnvalue)))
      (bind _returnvalue_2 (Game|GetCurrentLevelName true))
      (Game|OpenLevel(byName) (Utilities|String|StringToName _returnvalue_2))
      (else
        (Game|OpenLevel(byName) "Mainmenu")))))

(event Input|EnhancedActionEvents|EnhancedInputActionIA_Move
  (params (ActionValue :type Vector%202D%20Structure) (ElapsedSeconds :type Float%20%28double-precision%29) (TriggeredSeconds :type Float%20%28double-precision%29) (InputAction :type Input%20Action%20Object%20Reference :default "/Game/Input/IA_Move.IA_Move"))
  (:Triggered
    (Variables|Default|SetMoveInput ActionValue))
  (:Completed
    (Variables|Default|SetMoveInput "")))

(event EventBeginPlay
  (bind _output_get (Variables|Default|SetMAX_HP (Variables|/Game/Data/PDA_PlayerStats.PDA_PlayerStats_C|GetMAX_HP (Variables|Default|GetStats))))
  (Variables|Default|SetHP _output_get)
  (Input|AddMappingContext (PlayerController|LocalPlayerSubsystems|GetEnhancedInputLocalPlayerSubsystem (Game|GetPlayerController 0)) "/Game/Input/IMC_Car.IMC_Car" 0 "(bIgnoreAllPressedKeysUntilRelease=True,bForceImmediately=False,bNotifyUserSettings=False)")
  (bind _returnvalue (UserInterface|CreateWidget "/Game/Levels/BP_HUD.BP_HUD_C"))
  (UserInterface|Viewport|AddtoViewport _returnvalue 0)
  (bind _output_get_2 (Variables|Default|SetHUDRef _returnvalue))
  (bind _output_get_3 (Variables|Default|SetCoinsLeft (Variables|/Script/Racescape.LevelData|GetGoalCoins (Variables|/Script/Racescape.SaveSubsystem|GetSelectedLevel (Subsystems|GetSaveSubsystem)))))
  (Default|UpdateCoins _output_get_2 _output_get_3)
  (Default|UpdateHP (Variables|Default|GetHUDRef) (Variables|Default|GetHP) (Variables|Default|GetMAX_HP))
  (if (<= (Variables|Default|GetHP) 0.0)
    (bind _returnvalue_2 (Game|GetCurrentLevelName true))
    (Game|OpenLevel(byName) (Utilities|String|StringToName _returnvalue_2))))

(event Collision|EventActorBeginOverlap
  (params (OtherActor :type Actor%20Object%20Reference)))

(event EventTick
  (params (DeltaSeconds :type Float%20%28single-precision%29))
  (bind _moveinput (Variables|Default|GetMoveInput))
  (bind _stats (Variables|Default|GetStats))
  (bind (_x _y) (Math|Vector2D|BreakVector2D _moveinput))
  (bind _returnvalue (Math|Vector|MakeVector _y _x 0.0))
  (Utilities|FlowControl|Sequence
    (:then_0
      (Pawn|Input|AddMovementInput _returnvalue 1.0 false)
      (if (> (Math|Vector|VectorLength _returnvalue) 0.1)
        (Transformation|SetActorRotation (Math|Interpolation|RInterpTo (Transformation|GetActorRotation) (Math|Rotator|MakeRotfromX _returnvalue) DeltaSeconds 8.0))))
    (:then_1
      (Variables|Default|SetVerticalSpeed (- (Variables|Default|GetVerticalSpeed) (* DeltaSeconds (Variables|/Game/Data/PDA_PlayerStats.PDA_PlayerStats_C|GetGravity _stats))))
      (bind _sweephitresult (Transformation|AddActorWorldOffset (Math|Vector|MakeVector 0.0 0.0 (* DeltaSeconds (Variables|Default|GetVerticalSpeed))) true))
      (if (.bBlockingHit (Collision|BreakHitResult _sweephitresult))
        (Variables|Default|SetVerticalSpeed (Variables|/Game/Data/PDA_PlayerStats.PDA_PlayerStats_C|GetTurnInterpSpeed _stats))))))

(event Game|Damage|EventAnyDamage
  (params (Damage :type Float%20%28single-precision%29) (DamageType :type Damage%20Type%20Object%20Reference) (InstigatedBy :type Controller%20Object%20Reference) (DamageCauser :type Actor%20Object%20Reference))
  (Variables|Default|SetHP (Math|Float|Clamp(Float) (- (Variables|Default|GetHP) Damage) 0.0 (Variables|Default|GetMAX_HP)))
  (Default|UpdateHP (Variables|Default|GetHUDRef) (Variables|Default|GetHP) (Variables|Default|GetMAX_HP))
  (if (<= (Variables|Default|GetHP) 0.0)
    (bind _returnvalue (Game|GetCurrentLevelName true))
    (Game|OpenLevel(byName) (Utilities|String|StringToName _returnvalue))))

(fn ConstructionScript)